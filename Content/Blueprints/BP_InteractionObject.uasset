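; BP_InteractionObject is an interactable actor that shows a use-icon billboard as a prompt to the first-person player.
; Overlap begin and end with BP_FirstPersonCharacter show and hide the billboard.
; Each Tick looks up the character and compares its distance to ActiveDistance, switching the icon's ColorTint between proximity and original colors through a dynamic material created at BeginPlay.
; It only handles this visual feedback, with no use action.
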(event `self.ReceiveBeginPlay`
  (bind _returnvalue (`PrimitiveComponent.CreateDynamicMaterialInstance` (`self.MaterialBillboard`) 0 "/Game/Textures/MAT_use-icon.MAT_use-icon" "None")))

(event `self.ReceiveTick`
  (params (DeltaSeconds :type "Float (single-precision)"))
  ;[1 1 1] check if player is close enough to use the object
  (bind _returnvalue (`GameplayStatics.GetActorOfClass` "/Game/FirstPerson/Blueprints/BP_FirstPersonCharacter.BP_FirstPersonCharacter_C"))
  (if (< (`KismetMathLibrary.Vector_Distance` (`self.K2_GetActorLocation`) (`self.K2_GetActorLocation` _returnvalue)) (`self.ActiveDistance`))
    (`MaterialInstanceDynamic.SetVectorParameterValue` (stale `self.ReceiveBeginPlay` _returnvalue) "ColorTint" (`KismetMathLibrary.Conv_ColorToLinearColor` (`self.ProximityColor`)))
    (else
      (`MaterialInstanceDynamic.SetVectorParameterValue` (stale `self.ReceiveBeginPlay` _returnvalue) "ColorTint" (`KismetMathLibrary.Conv_ColorToLinearColor` (`self.OriginalColor`))))))

(event `self.ReceiveActorBeginOverlap`
  (params (OtherActor :type "Actor Object Reference"))
  ;[1 1 1] only react to the player actor
  (cast `/Game/FirstPerson/Blueprints/BP_FirstPersonCharacter` OtherActor)
  (`SceneComponent.SetVisibility` (`self.MaterialBillboard`) true false))

(event `self.ReceiveActorEndOverlap`
  (params (OtherActor :type "Actor Object Reference"))
  ;[1 1 1] only react to the player actor
  (cast `/Game/FirstPerson/Blueprints/BP_FirstPersonCharacter` OtherActor)
  (`SceneComponent.SetVisibility` (`self.MaterialBillboard`) false false))

(fn `UserConstructionScript`)
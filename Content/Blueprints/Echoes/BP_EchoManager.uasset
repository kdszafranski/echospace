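; Echo manager that records the player's runs and replays them as BP_Echo actors when the player restarts.
; Tick advances a turn timer and, throttled by a half-second Delay, stores position snapshots; action snapshots can also carry a target object.
; Finalizing moves the snapshots into EchoList.
; Restarting returns the player to the saved start, zeroes the timer, respawns every echo and resets door switches.
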(event `SavePlayerStart`
  ;[1 1 1] store reference to player
  (bind _returnvalue (`GameplayStatics.GetActorOfClass` "/Game/FirstPerson/Blueprints/BP_FirstPersonCharacter.BP_FirstPersonCharacter_C"))
  (bind _output_get (set `self.CurrentPlayer` _returnvalue))
  (set `self.PlayerStartingLocation` (`self.K2_GetActorLocation` _output_get))
  (set `self.PlayerStartingRotation` (`Pawn.GetControlRotation` _output_get)))

(event `self.ReceiveTick`
  (params (DeltaSeconds :type "Float (single-precision)"))
  ;[1 1 1] Store Player position and target snapshots for later playback by an Echo
  (set `self.CurrentTurnTimer` (+ DeltaSeconds (`self.CurrentTurnTimer`)))
  (`KismetSystemLibrary.Delay` 0.5)
  (`self.OnTakeSnapshot` null))

(event `OnTakeSnapshot`
  (params (ActionTargetObject :type "Object Object Reference") (MoveIndex :type Integer))
  ;[1 1 1] Stores player position and event object (if provided)
  (`self.StoreSnapshot` (make `/Game/Blueprints/Echoes/ST_SnapshotData` (`self.K2_GetActorLocation` (`self.CurrentPlayer`)) ActionTargetObject (`self.CurrentTurnTimer`) MoveIndex)))

(event `OnFinalizeEchoData`
  ;[1 1 1] Records Event object into snapshots then clears snapshots so we can restart player
  (`KismetArrayLibrary.Array_Add` (`self.EchoList`) (make `/Game/Blueprints/Echoes/ST_Echo` (`self.SnapshotList`)))
  (`KismetArrayLibrary.Array_Clear` (`self.SnapshotList`)))

(event `OnSpawnAllEchoes`
  ;[1 1 1] goes thru echo array and turns each one into an Echo in the scene
  (bind _outactors (`GameplayStatics.GetAllActorsOfClass` "/Game/Blueprints/Echoes/BP_Echo.BP_Echo_C"))
  ;[1 1 1] destroy existing echoes in scene
  (for _array_element _outactors
    (`self.K2_DestroyActor` _array_element))
  ;[1 1 1] spawn new echoes
  (for _array_element_2 (`self.EchoList`)
    (`self.SpawnEcho` _array_element_2))
  ;[1 1 1] reset door switches
  (bind _outactors_2 (`GameplayStatics.GetAllActorsOfClass` "/Game/Blueprints/LevelObjects/Level0/BP_DoorSwitch.BP_DoorSwitch_C"))
  (for _array_element_3 _outactors_2
    (`/Game/Blueprints/LevelObjects/Level0/BP_DoorSwitch.ResetHandle` _array_element_3)))

(event `RestartPlayer`
  (bind _currentplayer (`self.CurrentPlayer`))
  ;[1 1 1] Reset Player position and rotation
  (`self.K2_SetActorLocation` _currentplayer (`self.PlayerStartingLocation`) false false)
  (`Controller.SetControlRotation` (`Pawn.GetController` _currentplayer) (`self.PlayerStartingRotation`))
  ;;[1 0.3985 0.0625] Reset the turn timer so the next echo uses this time as the basis instead of the game running time
  (set `self.CurrentTurnTimer` 0.0)
  (`self.OnSpawnAllEchoes`))

(fn `CreateSnapshot`
  (params (Location :type "Vector Structure") (DoorTarget :type "/Game/Blueprints/LevelObjects/Level0/BP_Doorway Object Reference"))
  ;[1 1 1] Called from PlayerCharacter when lever is pulled
  (`self.StoreSnapshot` (make `/Game/Blueprints/Echoes/ST_SnapshotData` Location DoorTarget (`KismetSystemLibrary.GetGameTimeInSeconds`))))

(fn `SpawnEcho`
  (params (EchoData :type "/Game/Blueprints/Echoes/ST_Echo Structure"))
  (bind _snapshots (break `/Game/Blueprints/Echoes/ST_Echo` EchoData))
  ;[1 1 1] spawn at first saved position
  (bind _returnvalue (`|SpawnActorFromClass` "/Game/Blueprints/Echoes/BP_Echo.BP_Echo_C" (`KismetMathLibrary.MakeTransform` (`.Location_2_EDFC858F49A13C15039BC1BD7EC124C6` (break `/Game/Blueprints/Echoes/ST_SnapshotData` (`|GetArrayItem` _snapshots)))) "Undefined" "MultiplyWithRoot" null null))
  ;[1 1 1] initialize
  (`/Game/Blueprints/Echoes/BP_Echo.OnSpawned` _returnvalue _snapshots))

(fn `StoreEcho`
  (params (SnapshotList :type "Array of /Game/Blueprints/Echoes/ST_SnapshotData Structure")))

(fn `StoreSnapshot`
  (params (Snapshot :type "/Game/Blueprints/Echoes/ST_SnapshotData Structure"))
  ;[1 1 1] Adds this snapshot to the array
  (`KismetArrayLibrary.Array_Add` (`self.SnapshotList`) Snapshot))

(fn `UserConstructionScript`)
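; BP_EchoManager records the player's movements and actions and replays them as Echo actors.
; A delayed Tick samples player location about every half second, while CreateSnapshot adds timestamped lever actions with their door targets.
; OnStoreAction saves the snapshots as an Echo, clears them and returns the player to the starting transform.
; OnSpawnAllEchoes spawns a BP_EchoWithAnimation at each recording's first location and passes it the snapshots.
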(event `self.ReceiveBeginPlay`
  ;[1 1 1] store reference to player
  (bind _returnvalue (`GameplayStatics.GetActorOfClass` "/Game/FirstPerson/Blueprints/BP_FirstPersonCharacter.BP_FirstPersonCharacter_C"))
  (bind _output_get (set `self.CurrentPlayer` _returnvalue))
  (set `self.PlayerStartingLocation` (`self.K2_GetActorLocation` _output_get))
  (set `self.PlayerStartingRotation` (`self.K2_GetActorRotation` _output_get)))

(event `self.ReceiveTick`
  (params (DeltaSeconds :type "Float (single-precision)"))
  ;[1 1 1] Store position and target snapshots for later playback by an Echo
  (`KismetSystemLibrary.Delay` 0.5)
  (`self.OnTakeSnapshot` null))

(event `OnTakeSnapshot`
  (params (DoorTarget :type "Object Object Reference") (MoveIndex :type Integer))
  (`self.StoreSnapshot` (make `/Game/Blueprints/SnapshotData` (`self.K2_GetActorLocation` (`self.CurrentPlayer`)) DoorTarget (`KismetSystemLibrary.GetGameTimeInSeconds`) MoveIndex)))

(event `OnStoreAction`
  ;[1 1 1] Store current snapshots as a new Echo struct, then clear snapshots and reset player
  (`KismetArrayLibrary.Array_Add` (`self.EchoList`) (make `/Game/Blueprints/ST_Echo` (`self.SnapshotList`)))
  (`KismetArrayLibrary.Array_Clear` (`self.SnapshotList`))
  (`self.K2_SetActorLocationAndRotation` (`self.CurrentPlayer`) (`self.PlayerStartingLocation`) (`self.PlayerStartingRotation`) false false))

(event `OnSpawnAllEchoes`
  ;[1 1 1] goes thru echo array and turns each one into an Echo in the scene
  (for _array_element (`self.EchoList`)
    (`self.SpawnEcho` _array_element)))

(event `OnEventWasTriggered`
  (set `self.EventTime` (`self.GetGameTimeSinceCreation`)))

(fn `CreateSnapshot`
  (params (Location :type "Vector Structure") (DoorTarget :type "/Game/Blueprints/LevelObjects/Level0/BP_Doorway Object Reference"))
  ;[1 1 1] Called from PlayerCharacter when lever is pulled
  (`self.StoreSnapshot` (make `/Game/Blueprints/SnapshotData` Location DoorTarget (`KismetSystemLibrary.GetGameTimeInSeconds`))))

(fn `SpawnEcho`
  (params (EchoData :type "/Game/Blueprints/ST_Echo Structure"))
  (bind _snapshots (break `/Game/Blueprints/ST_Echo` EchoData))
  (`KismetSystemLibrary.PrintString` "spawning echo BP")
  ;[1 1 1] spawn at first saved position
  (bind _returnvalue (`|SpawnActorFromClass` "/Game/Blueprints/BP_EchoWithAnimation.BP_EchoWithAnimation_C" (`KismetMathLibrary.MakeTransform` (`.Location_2_EDFC858F49A13C15039BC1BD7EC124C6` (break `/Game/Blueprints/SnapshotData` (`|GetArrayItem` _snapshots)))) "Undefined" "MultiplyWithRoot" null null))
  ;[1 1 1] initialize
  (`/Game/Blueprints/BP_Echo.OnSpawned` _returnvalue _snapshots))

(fn `StoreEcho`
  (params (SnapshotList :type "Array of /Game/Blueprints/SnapshotData Structure")))

(fn `StoreSnapshot`
  (params (Snapshot :type "/Game/Blueprints/SnapshotData Structure"))
  (`KismetArrayLibrary.Array_Add` (`self.SnapshotList`) Snapshot))

(fn `UserConstructionScript`)
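; Puzzle lever that sends its stored location to the mover manager when its action is performed.
; PerformAction calls CallMover, which, if the lever is enabled, finds BP_MoverManager with GetActorOfClass and passes MyLocation to SetMoveLocation.
; The trailing delay leads to nothing, and the nodes that would rotate the lever mesh are disconnected, so the graph does not animate the lever.
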(event `/Game/Blueprints/BPI_Actions.PerformAction`
  ;[0 1 0.1856] TAKE ACTION
  (`self.CallMover`)
  (`KismetSystemLibrary.Delay` 0.6))

(event `CallMover`
  (if (`self.enabled`)
    (bind _returnvalue (`GameplayStatics.GetActorOfClass` "/Game/Blueprints/LevelObjects/BP_MoverManager.BP_MoverManager_C"))
    (`/Game/Blueprints/LevelObjects/BP_MoverManager.SetMoveLocation` _returnvalue (`self.myLocation`))))

(fn `UserConstructionScript`)
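; BP_PuzzleLargeControl1 is a puzzle control that nudges one bar of its puzzle's guess up or down when activated.
; Activate, ignored while disabled or locked, calls AdjustGuess on MyPuzzle, spawns a lever sound actor and briefly flashes the slider material.
; Disable and Reenable toggle input, while Lock permanently disables it, spawns a row-lock actor and propagates to its sibling control, guarded against repeat calls.
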(event `Activate`
  (bind _slidersmall_1l (`self.sliderSmall_1l`))
  (if (`self.disabled`)
    _
    (elif (not (`self.locked`))
      (`/Game/Blueprints/Puzzles/BP_PuzzleSliderLarge.AdjustGuess` (`self.MyPuzzle`) (`self.Bar`) (`self.Up`) self)
      (`|SpawnActorFromClass` "/Game/Blueprints/Audio/BP_LeverPullSound.BP_LeverPullSound_C" (`KismetMathLibrary.MakeTransform` (`SceneComponent.K2_GetComponentLocation` (`self.DefaultSceneRoot`))) "Undefined" "MultiplyWithRoot" null null)
      (`PrimitiveComponent.SetMaterial` _slidersmall_1l 0 "/Game/Materials00/MT_SliderLocked.MT_SliderLocked")
      (`KismetSystemLibrary.Delay` 0.1)
      (`PrimitiveComponent.SetMaterial` _slidersmall_1l 0 "/Game/StarterContent/Materials/M_Metal_Brushed_Nickel.M_Metal_Brushed_Nickel"))))

(event `Disable`
  (set `self.disabled` true))

(event `Reenable`
  (set `self.disabled` false))

(event `Lock`
  (if (not (`self.locked`))
    (`self.Disable`)
    (set `self.locked` true)
    (`|SpawnActorFromClass` "/Game/Sound/BP_PuzzleRowLock.BP_PuzzleRowLock_C" (`KismetMathLibrary.MakeTransform` (`SceneComponent.K2_GetComponentLocation` (`self.DefaultSceneRoot`))) "Undefined" "MultiplyWithRoot" null null)
    (`self.Lock` (`self.mySibling`))))

(fn `UserConstructionScript`)
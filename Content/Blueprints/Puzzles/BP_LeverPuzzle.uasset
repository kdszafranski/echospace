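; BP_LeverPuzzle is a puzzle lever actor that rotates its lever mesh when an action is performed on it.
; PerformAction calls SolvePuzzle, then logs itself as the trigger to the BP_ActionsManager found in the level, with zero time and ghost index.
; SolvePuzzle picks one of two pitch rotations from Toggled, but each branch writes back the same value, so the state never flips.
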(event `/Game/Blueprints/BPI_Actions.PerformAction`
  ;[0 1 0.1856] TAKE ACTION
  (`self.SolvePuzzle`)
  (bind _returnvalue (`GameplayStatics.GetActorOfClass` "/Game/Blueprints/BP_ActionsManager.BP_ActionsManager_C"))
  (`/Game/Blueprints/BP_ActionsManager.LogAction` _returnvalue self 0.0 0))

(event `SolvePuzzle`
  (bind _lever00_cube_001 (`self.lever00_Cube_001`))
  (if (`self.toggled`)
    (`SceneComponent.K2_SetRelativeRotation` _lever00_cube_001 (`KismetMathLibrary.MakeRotator` 0.0) false false)
    (set `self.toggled` true)
    (else
      (`SceneComponent.K2_SetRelativeRotation` _lever00_cube_001 (`KismetMathLibrary.MakeRotator` 0.0 90.0) false false)
      (set `self.toggled` false))))

(fn `UserConstructionScript`)
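; Three-slider puzzle actor that randomizes three target values on BeginPlay and places hint indicators to show them.
; AdjustGuess steps the indexed guess up or down, and AdjustSliders repositions the indicator cubes to match.
; A guess within tolerance locks the passed button and applies the locked material to that slider.
; Three matches stop the alarm and call SolvePuzzle on BP_PuzzleManager; LockPlacement is empty and ShowHint is uncalled here.
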(event `self.ReceiveBeginPlay`
  (bind _hintindicator2 (`self.hintIndicator2`))
  (bind _indicatorminy (`self.indicatorMinY`))
  (bind _hintindicator1 (`self.hintIndicator1`))
  (bind _hintindicator0 (`self.hintIndicator0`))
  (bind _indicatormaxy (`self.indicatorMaxY`))
  (bind (_relativelocation_x _relativelocation_y _relativelocation_z) (`KismetMathLibrary.BreakVector` (`SceneComponent.RelativeLocation` _hintindicator0)))
  (bind (_relativelocation_x_2 _relativelocation_y_2 _relativelocation_z_2) (`KismetMathLibrary.BreakVector` (`SceneComponent.RelativeLocation` _hintindicator1)))
  (bind (_relativelocation_x_3 _relativelocation_y_3 _relativelocation_z_3) (`KismetMathLibrary.BreakVector` (`SceneComponent.RelativeLocation` _hintindicator2)))
  (set `self.value0` (`KismetMathLibrary.RandomFloat`))
  (set `self.value1` (`KismetMathLibrary.RandomFloat`))
  (set `self.value2` (`KismetMathLibrary.RandomFloat`))
  ;[0 1 0.9064] Hint0
  (`SceneComponent.K2_SetRelativeLocation` _hintindicator0 (`KismetMathLibrary.MakeVector` _relativelocation_x (+ (* (`self.value0`) (- _indicatormaxy _indicatorminy)) _indicatorminy) _relativelocation_z) false false)
  ;[0 1 0.9064] Hint1
  (`SceneComponent.K2_SetRelativeLocation` _hintindicator1 (`KismetMathLibrary.MakeVector` _relativelocation_x_2 (+ (* (`self.value1`) (- _indicatormaxy _indicatorminy)) _indicatorminy) _relativelocation_z_2) false false)
  ;[0 1 0.9064] Hint2
  (`SceneComponent.K2_SetRelativeLocation` _hintindicator2 (`KismetMathLibrary.MakeVector` _relativelocation_x_3 (+ (* (`self.value2`) (- _indicatormaxy _indicatorminy)) _indicatorminy) _relativelocation_z_3) false false)
  (`self.AdjustSliders`))

(event `LockPlacement`)

(event `AdjustSliders`
  (bind _guessmaxy (`self.guessMaxY`))
  (bind _sliderlarge_indicatorcube0 (`self.sliderLarge_indicatorCube0`))
  (bind _sliderlarge_indicatorcube1 (`self.sliderLarge_indicatorCube1`))
  (bind _sliderlarge_indicatorcube2 (`self.sliderLarge_indicatorCube2`))
  (bind _guessminy (`self.guessMinY`))
  (bind (_relativelocation_x _relativelocation_y _relativelocation_z) (`KismetMathLibrary.BreakVector` (`SceneComponent.RelativeLocation` _sliderlarge_indicatorcube0)))
  (bind (_relativelocation_x_2 _relativelocation_y_2 _relativelocation_z_2) (`KismetMathLibrary.BreakVector` (`SceneComponent.RelativeLocation` _sliderlarge_indicatorcube1)))
  (bind (_relativelocation_x_3 _relativelocation_y_3 _relativelocation_z_3) (`KismetMathLibrary.BreakVector` (`SceneComponent.RelativeLocation` _sliderlarge_indicatorcube2)))
  ;[0 1 0.8465] Comment
  (`SceneComponent.K2_SetRelativeLocation` _sliderlarge_indicatorcube0 (`KismetMathLibrary.MakeVector` _relativelocation_x (+ (* (`self.Guess0`) (- _guessmaxy _guessminy)) _guessminy) _relativelocation_z) false false)
  (`SceneComponent.K2_SetRelativeLocation` _sliderlarge_indicatorcube1 (`KismetMathLibrary.MakeVector` _relativelocation_x_2 (+ (* (`self.Guess1`) (- _guessmaxy _guessminy)) _guessminy) _relativelocation_z_2) false false)
  (`SceneComponent.K2_SetRelativeLocation` _sliderlarge_indicatorcube2 (`KismetMathLibrary.MakeVector` _relativelocation_x_3 (+ (* (`self.Guess2`) (- _guessmaxy _guessminy)) _guessminy) _relativelocation_z_3) false false))

(event `AdjustGuess`
  (params (GuessIndex :type Integer) (Up :type Boolean) (Button :type "/Game/Blueprints/Puzzles/BP_PuzzleSmallControl Object Reference"))
  (bind _guess0 (`self.Guess0`))
  (bind _step (`self.Step`))
  (bind _guess1 (`self.Guess1`))
  (bind _guess2 (`self.Guess2`))
  ;[0 1 0.9725] working
  (if (== GuessIndex 0)
    (if Up
      (if (< _guess0 0.9)
        (set `self.Guess0` (+ _guess0 _step))
        (`self.AdjustSliders` :!label _label)
        (if (< (`KismetMathLibrary.Abs` (- (`self.value0`) (`self.Guess0`))) (/ (`self.Step`) 1.5))
          (`/Game/Blueprints/Puzzles/BP_PuzzleSmallControl.Lock` Button)
          (bind _output_get (set `self.solvedMaterial` "/Game/Materials00/MT_SliderLocked.MT_SliderLocked"))
          (`PrimitiveComponent.SetMaterial` (`self.hintIndicator0`) 0 _output_get)
          (`PrimitiveComponent.SetMaterial` (`self.sliderLarge_indicatorCube0`) 0 _output_get)
          (`PrimitiveComponent.SetMaterial` (`self.sliderLarge_correctCube0`) 0 _output_get)
          (bind _output_get_2 (set `self.solvedCount` (+ (`self.solvedCount`) 1) :!label _label_2))
          (if (>= _output_get_2 3)
            (`PrimitiveComponent.SetMaterial` (`self.sliderLarge_correctCube3`) 0 _output_get)
            (`AudioComponent.Stop` (`self.SND_Alarm`))
            (bind _returnvalue (`GameplayStatics.GetActorOfClass` "/Game/Blueprints/Puzzles/BP_PuzzleManager.BP_PuzzleManager_C"))
            (`/Game/Blueprints/Puzzles/BP_PuzzleManager.SolvePuzzle` _returnvalue))))
      (elif (> _guess0 _step)
        (set `self.Guess0` (- _guess0 _step))
        (goto _label)))
    (elif (== GuessIndex 1)
      (if Up
        (if (< _guess1 0.9)
          (set `self.Guess1` (+ _guess1 _step))
          (`self.AdjustSliders` :!label _label_3)
          (if (< (`KismetMathLibrary.Abs` (- (`self.value1`) (`self.Guess1`))) (/ (`self.Step`) 1.5))
            (`/Game/Blueprints/Puzzles/BP_PuzzleSmallControl.Lock` Button)
            (bind _output_get_3 (set `self.solvedMaterial` "/Game/Materials00/MT_SliderLocked.MT_SliderLocked"))
            (`PrimitiveComponent.SetMaterial` (`self.hintIndicator1`) 0 _output_get_3)
            (`PrimitiveComponent.SetMaterial` (`self.sliderLarge_indicatorCube1`) 0 _output_get_3)
            (`PrimitiveComponent.SetMaterial` (`self.sliderLarge_correctCube1`) 0 _output_get_3)
            (goto _label_2)))
        (elif (> _guess1 _step)
          (set `self.Guess1` (- _guess1 _step))
          (goto _label_3)))
      (elif Up
        (if (< _guess2 0.9)
          (set `self.Guess2` (+ _guess2 _step))
          (`self.AdjustSliders` :!label _label_4)
          (if (< (`KismetMathLibrary.Abs` (- (`self.value2`) (`self.Guess2`))) (/ (`self.Step`) 1.5))
            (`/Game/Blueprints/Puzzles/BP_PuzzleSmallControl.Lock` Button)
            (bind _output_get_4 (set `self.solvedMaterial` "/Game/Materials00/MT_SliderLocked.MT_SliderLocked"))
            (`PrimitiveComponent.SetMaterial` (`self.hintIndicator2`) 0 _output_get_4)
            (`PrimitiveComponent.SetMaterial` (`self.sliderLarge_indicatorCube2`) 0 _output_get_4)
            (`PrimitiveComponent.SetMaterial` (`self.sliderLarge_correctCube2`) 0 _output_get_4)
            (goto _label_2)))
        (elif (> _guess2 _step)
          (set `self.Guess2` (- _guess2 _step))
          (goto _label_4))))))

(fn `Show Hint`
  (params (Value :type "Float (double-precision)") (MiY :type "Float (double-precision)") (MaxY :type "Float (double-precision)") (Indicator :type "StaticMeshComponent Object Reference"))
  (bind (_relativelocation_x _relativelocation_y _relativelocation_z) (`KismetMathLibrary.BreakVector` (`SceneComponent.RelativeLocation` Indicator)))
  (`SceneComponent.K2_SetRelativeLocation` Indicator (`KismetMathLibrary.MakeVector` _relativelocation_x (+ (* Value (- MiY MaxY)) MaxY) _relativelocation_z) false false))

(fn `UserConstructionScript`)
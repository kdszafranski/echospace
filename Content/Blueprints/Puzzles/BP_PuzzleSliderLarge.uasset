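; Five-slider puzzle actor where each guess is nudged up or down to match a randomized target.
; BeginPlay rolls the targets and positions hint indicators; AdjustSliders maps guesses to cube positions.
; AdjustGuess steps one guess, finer for the fifth, and applies the locked material within tolerance without blocking further movement.
; Every in-tolerance adjustment increments SolvedCount, even repeats, and five lights the final correct cube; LockPlacement is empty.
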(event `self.ReceiveBeginPlay`
  (bind _indicatorminx (`self.indicatorMinX`))
  (bind _hintindicator2 (`self.hintIndicator2`))
  (bind _hintindicator1 (`self.hintIndicator1`))
  (bind _hintindicator0 (`self.hintIndicator0`))
  (bind _hintindicator3 (`self.hintIndicator3`))
  (bind _hintindicator4 (`self.hintIndicator4`))
  (bind _indicatormaxx (`self.indicatorMaxX`))
  (bind (_relativelocation_x _relativelocation_y _relativelocation_z) (`KismetMathLibrary.BreakVector` (`SceneComponent.RelativeLocation` _hintindicator0)))
  (bind (_relativelocation_x_2 _relativelocation_y_2 _relativelocation_z_2) (`KismetMathLibrary.BreakVector` (`SceneComponent.RelativeLocation` _hintindicator1)))
  (bind (_relativelocation_x_3 _relativelocation_y_3 _relativelocation_z_3) (`KismetMathLibrary.BreakVector` (`SceneComponent.RelativeLocation` _hintindicator4)))
  (bind (_relativelocation_x_4 _relativelocation_y_4 _relativelocation_z_4) (`KismetMathLibrary.BreakVector` (`SceneComponent.RelativeLocation` _hintindicator2)))
  (bind (_relativelocation_x_5 _relativelocation_y_5 _relativelocation_z_5) (`KismetMathLibrary.BreakVector` (`SceneComponent.RelativeLocation` _hintindicator3)))
  (set `self.value0` (`KismetMathLibrary.RandomFloat`))
  (set `self.value1` (`KismetMathLibrary.RandomFloat`))
  (set `self.value2` (`KismetMathLibrary.RandomFloat`))
  (set `self.value3` (`KismetMathLibrary.RandomFloat`))
  (set `self.value4` (`KismetMathLibrary.RandomFloat`))
  ;[0 1 0.9064] Hint0
  (`SceneComponent.K2_SetRelativeLocation` _hintindicator0 (`KismetMathLibrary.MakeVector` _relativelocation_x (+ (* (`self.value0`) (- _indicatormaxx _indicatorminx)) _indicatorminx) _relativelocation_z) false false)
  ;[0 1 0.9064] Hint1
  (`SceneComponent.K2_SetRelativeLocation` _hintindicator1 (`KismetMathLibrary.MakeVector` _relativelocation_x_2 (+ (* (`self.value1`) (- _indicatormaxx _indicatorminx)) _indicatorminx) _relativelocation_z_2) false false)
  ;[0 1 0.9064] Hint2
  (`SceneComponent.K2_SetRelativeLocation` _hintindicator2 (`KismetMathLibrary.MakeVector` _relativelocation_x_4 (+ (* (`self.value2`) (- _indicatormaxx _indicatorminx)) _indicatorminx) _relativelocation_z_4) false false)
  ;[0 1 0.9064] Hint3
  (`SceneComponent.K2_SetRelativeLocation` _hintindicator3 (`KismetMathLibrary.MakeVector` _relativelocation_x_5 (+ (* (`self.value3`) (- _indicatormaxx _indicatorminx)) _indicatorminx) _relativelocation_z_5) false false)
  ;[0 1 0.9064] Hint4
  (`SceneComponent.K2_SetRelativeLocation` _hintindicator4 (`KismetMathLibrary.MakeVector` _relativelocation_x_3 (+ (* (`self.value4`) (- _indicatormaxx _indicatorminx)) _indicatorminx) _relativelocation_z_3) false false)
  (`self.AdjustSliders`))

(event `LockPlacement`)

(event `AdjustSliders`
  (bind _guessmaxx (`self.guessMaxX`))
  (bind _sliderlarge_indicatorcube0 (`self.sliderLarge_indicatorCube0`))
  (bind _sliderlarge_indicatorcube1 (`self.sliderLarge_indicatorCube1`))
  (bind _guessminx (`self.guessMinX`))
  (bind _sliderlarge_indicatorcube2 (`self.sliderLarge_indicatorCube2`))
  (bind _sliderlarge_indicatorcube3 (`self.sliderLarge_indicatorCube3`))
  (bind _sliderlarge_indicatorcube4 (`self.sliderLarge_indicatorCube4`))
  (bind (_relativelocation_x _relativelocation_y _relativelocation_z) (`KismetMathLibrary.BreakVector` (`SceneComponent.RelativeLocation` _sliderlarge_indicatorcube0)))
  (bind (_relativelocation_x_2 _relativelocation_y_2 _relativelocation_z_2) (`KismetMathLibrary.BreakVector` (`SceneComponent.RelativeLocation` _sliderlarge_indicatorcube1)))
  (bind (_relativelocation_x_3 _relativelocation_y_3 _relativelocation_z_3) (`KismetMathLibrary.BreakVector` (`SceneComponent.RelativeLocation` _sliderlarge_indicatorcube4)))
  (bind (_relativelocation_x_4 _relativelocation_y_4 _relativelocation_z_4) (`KismetMathLibrary.BreakVector` (`SceneComponent.RelativeLocation` _sliderlarge_indicatorcube2)))
  (bind (_relativelocation_x_5 _relativelocation_y_5 _relativelocation_z_5) (`KismetMathLibrary.BreakVector` (`SceneComponent.RelativeLocation` _sliderlarge_indicatorcube3)))
  ;[0 1 0.8465] Comment
  (`SceneComponent.K2_SetRelativeLocation` _sliderlarge_indicatorcube0 (`KismetMathLibrary.MakeVector` _relativelocation_x (+ (* (`self.Guess0`) (- _guessmaxx _guessminx)) _guessminx) _relativelocation_z) false false)
  (`SceneComponent.K2_SetRelativeLocation` _sliderlarge_indicatorcube1 (`KismetMathLibrary.MakeVector` _relativelocation_x_2 (+ (* (`self.Guess1`) (- _guessmaxx _guessminx)) _guessminx) _relativelocation_z_2) false false)
  (`SceneComponent.K2_SetRelativeLocation` _sliderlarge_indicatorcube2 (`KismetMathLibrary.MakeVector` _relativelocation_x_4 (+ (* (`self.Guess2`) (- _guessmaxx _guessminx)) _guessminx) _relativelocation_z_4) false false)
  (`SceneComponent.K2_SetRelativeLocation` _sliderlarge_indicatorcube3 (`KismetMathLibrary.MakeVector` _relativelocation_x_5 (+ (* (`self.Guess3`) (- _guessmaxx _guessminx)) _guessminx) _relativelocation_z_5) false false)
  (`SceneComponent.K2_SetRelativeLocation` _sliderlarge_indicatorcube4 (`KismetMathLibrary.MakeVector` _relativelocation_x_3 (+ (* (`self.Guess4`) (- 113.0 -33.0)) -33.0) _relativelocation_z_3) false false))

(event `AdjustGuess`
  (params (GuessIndex :type Integer) (Up :type Boolean) (Button :type "/Game/Blueprints/Puzzles/BP_PuzzleLargeControl1 Object Reference"))
  (bind _guess4 (`self.Guess4`))
  (bind _guess0 (`self.Guess0`))
  (bind _step (`self.Step`))
  (bind _guess1 (`self.Guess1`))
  (bind _step_2 (`self.Step`))
  (bind _guess2 (`self.Guess2`))
  (bind _guess3 (`self.Guess3`))
  (bind _returnvalue (- 1.0 _step_2))
  (bind _returnvalue_2 (* _step 0.5))
  ;[0 1 0.9725] working
  (`KismetSystemLibrary.PrintString` "Adjust Guess")
  (if (== GuessIndex 0)
    (if Up
      (if (< _guess0 _returnvalue)
        (set `self.Guess0` (+ _guess0 _step))
        (`self.AdjustSliders` :!label _label)
        (if (<= (`KismetMathLibrary.Abs` (- (`self.value0`) (`self.Guess0`))) (`self.Step`))
          (bind _output_get (set `self.solvedMaterial` "/Game/Materials00/MT_SliderLocked.MT_SliderLocked"))
          (`PrimitiveComponent.SetMaterial` (`self.hintIndicator0`) 0 _output_get)
          (`PrimitiveComponent.SetMaterial` (`self.sliderLarge_indicatorCube0`) 0 _output_get)
          (`PrimitiveComponent.SetMaterial` (`self.correct0`) 0 _output_get)
          (bind _output_get_2 (set `self.solvedCount` (+ (`self.solvedCount`) 1) :!label _label_2))
          (if (>= _output_get_2 5)
            (`PrimitiveComponent.SetMaterial` (`self.sliderLarge_correctCube3`) 0 _output_get))))
      (elif (> _guess0 _step)
        (set `self.Guess0` (- _guess0 _step))
        (goto _label)))
    (elif (== GuessIndex 1)
      (if Up
        (if (< _guess1 _returnvalue)
          (set `self.Guess1` (+ _guess1 _step))
          (`self.AdjustSliders` :!label _label_3)
          (if (<= (`KismetMathLibrary.Abs` (- (`self.value1`) (`self.Guess1`))) (`self.Step`))
            (bind _output_get_3 (set `self.solvedMaterial` "/Game/Materials00/MT_SliderLocked.MT_SliderLocked"))
            (`PrimitiveComponent.SetMaterial` (`self.hintIndicator1`) 0 _output_get_3)
            (`PrimitiveComponent.SetMaterial` (`self.sliderLarge_indicatorCube1`) 0 _output_get_3)
            (`PrimitiveComponent.SetMaterial` (`self.correct1`) 0 _output_get_3)
            (goto _label_2)))
        (elif (> _guess1 _step)
          (set `self.Guess1` (- _guess1 _step))
          (goto _label_3)))
      (elif (== GuessIndex 2)
        (if Up
          (if (< _guess2 _returnvalue)
            (set `self.Guess2` (+ _guess2 _step))
            (`self.AdjustSliders` :!label _label_4)
            (if (<= (`KismetMathLibrary.Abs` (- (`self.value2`) (`self.Guess2`))) (`self.Step`))
              (bind _output_get_4 (set `self.solvedMaterial` "/Game/Materials00/MT_SliderLocked.MT_SliderLocked"))
              (`PrimitiveComponent.SetMaterial` (`self.hintIndicator2`) 0 _output_get_4)
              (`PrimitiveComponent.SetMaterial` (`self.sliderLarge_indicatorCube2`) 0 _output_get_4)
              (`PrimitiveComponent.SetMaterial` (`self.correct2`) 0 _output_get_4)
              (goto _label_2)))
          (elif (> _guess2 _step)
            (set `self.Guess2` (- _guess2 _step))
            (goto _label_4)))
        (elif (== GuessIndex 3)
          (if Up
            (if (< _guess3 (- 1.0 _step_2))
              (set `self.Guess3` (+ _guess3 _step))
              (`self.AdjustSliders` :!label _label_5)
              (if (<= (`KismetMathLibrary.Abs` (- (`self.value3`) (`self.Guess3`))) (`self.Step`))
                (bind _output_get_5 (set `self.solvedMaterial` "/Game/Materials00/MT_SliderLocked.MT_SliderLocked"))
                (`PrimitiveComponent.SetMaterial` (`self.hintIndicator3`) 0 _output_get_5)
                (`PrimitiveComponent.SetMaterial` (`self.sliderLarge_indicatorCube3`) 0 _output_get_5)
                (`PrimitiveComponent.SetMaterial` (`self.correct3`) 0 _output_get_5)
                (goto _label_2)))
            (elif (> _guess3 0.0)
              (set `self.Guess3` (- _guess3 _step))
              (goto _label_5)))
          (elif Up
            (if (< _guess4 (- 1.0 _returnvalue_2))
              (set `self.Guess4` (+ _guess4 _returnvalue_2))
              (`self.AdjustSliders` :!label _label_6)
              (if (<= (`KismetMathLibrary.Abs` (- (`self.value4`) (`self.Guess4`))) (* (`self.Step`) 0.5))
                (bind _output_get_6 (set `self.solvedMaterial` "/Game/Materials00/MT_SliderLocked.MT_SliderLocked"))
                (`PrimitiveComponent.SetMaterial` (`self.hintIndicator4`) 0 _output_get_6)
                (`PrimitiveComponent.SetMaterial` (`self.sliderLarge_indicatorCube4`) 0 _output_get_6)
                (`PrimitiveComponent.SetMaterial` (`self.correct4`) 0 _output_get_6)
                (goto _label_2)))
            (elif (> _guess4 0.0)
              (set `self.Guess4` (- _guess4 _returnvalue_2))
              (goto _label_6))))))))

(fn `Show Hint`
  (params (Value :type "Float (double-precision)") (MiY :type "Float (double-precision)") (MaxY :type "Float (double-precision)") (Indicator :type "StaticMeshComponent Object Reference"))
  (bind (_relativelocation_x _relativelocation_y _relativelocation_z) (`KismetMathLibrary.BreakVector` (`SceneComponent.RelativeLocation` Indicator)))
  (`SceneComponent.K2_SetRelativeLocation` Indicator (`KismetMathLibrary.MakeVector` _relativelocation_x (+ (* Value (- MiY MaxY)) MaxY) _relativelocation_z) false false))

(fn `UserConstructionScript`)
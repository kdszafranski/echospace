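; BP_PuzzleSmallControl is a puzzle button that nudges one entry of its parent puzzle's guess up or down.
; On Activate it passes its bar index, direction and itself to MyPuzzle.AdjustGuess, unless it is disabled or locked.
; Disable and Reenable toggle input, while Lock disables it and also sets a Locked flag that Reenable does not clear.
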(event `Activate`
  (if (`self.disabled`)
    _
    (elif (not (`self.locked`))
      (`/Game/Blueprints/Puzzles/BP_PuzzleSliderSmall.AdjustGuess` (`self.MyPuzzle`) (`self.Bar`) (`self.Up`) self))))

(event `Disable`
  (set `self.disabled` true))

(event `Reenable`
  (set `self.disabled` false))

(event `Lock`
  (`self.Disable`)
  (set `self.locked` true))

(fn `UserConstructionScript`)
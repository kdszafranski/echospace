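; BP_PistonController is a level object that drives a piston motion on the referenced MyCuff actor.
; On BeginPlay it stores the cuff's root location, then a timeline offsets that root along world X by the Piston track scaled by MoveDelta.
; When the timeline finishes it replays from the start, so the motion loops continuously without Tick.
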(event `self.ReceiveBeginPlay`
  (bind _mycuff (`self.MyCuff`))
  (bind (_startpos_x _startpos_y _startpos_z) (`KismetMathLibrary.BreakVector` (`self.StartPos`)))
  (bind _defaultsceneroot (`/Game/Blueprints/LevelObjects/BP_PistonCuff.DefaultSceneRoot` _mycuff))
  (set `self.StartPos` (`SceneComponent.K2_GetComponentLocation` (`/Game/Blueprints/LevelObjects/BP_PistonCuff.DefaultSceneRoot` _mycuff)))
  (bind (_direction _piston) (`Timeline|Timeline` :!label _label)
    (:`Update`
      (`SceneComponent.K2_SetWorldLocation` _defaultsceneroot (`KismetMathLibrary.MakeVector` (+ _startpos_x (* _piston (`self.MoveDelta`))) _startpos_y _startpos_z) false false))
    (:`Finished`
      (`SceneComponent.K2_SetWorldLocation` _defaultsceneroot (`SceneComponent.K2_GetComponentLocation` _defaultsceneroot) false false)
      (goto _label :!via `PlayFromStart`))))

(fn `UserConstructionScript`)
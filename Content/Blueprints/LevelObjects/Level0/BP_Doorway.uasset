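; BP_Doorway is a level doorway whose two door components swing open and then close automatically.
; The Open event plays a timeline that lerps both doors' relative yaw to a quarter turn, waits briefly, then calls Close.
; Close plays a second timeline that rotates them back, and both events print debug messages.
; Nothing connected in this graph triggers Open, as its delayed call is unwired and BeginPlay is empty.
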(event `self.ReceiveBeginPlay`)

(event `Open`
  (`KismetSystemLibrary.PrintString` "opening door")
  (bind (_direction _pistonopen) (`Timeline|OpenTimeline` :!via `PlayFromStart`)
    (:`Update`
      (bind _returnvalue (`KismetMathLibrary.Lerp` 0.0 90.0 _pistonopen))
      (`SceneComponent.K2_SetRelativeRotation` (`self.door2_Door1`) (`KismetMathLibrary.MakeRotator` 0.0 0.0 _returnvalue) false false)
      (`SceneComponent.K2_SetRelativeRotation` (`self.door2_Door2`) (`KismetMathLibrary.MakeRotator` 0.0 0.0 _returnvalue) false false))
    (:`Finished`
      (`KismetSystemLibrary.Delay` 3.0)
      (`self.Close`))))

(event `Close`
  (`KismetSystemLibrary.PrintString` "Closing Door")
  (bind (_direction _closer) (`Timeline|CloseTimeline` :!via `PlayFromStart`)
    (:`Update`
      (bind _returnvalue (`KismetMathLibrary.Lerp` 90.0 0.0 _closer))
      (`SceneComponent.K2_SetRelativeRotation` (`self.door2_Door1`) (`KismetMathLibrary.MakeRotator` 0.0 0.0 _returnvalue) false false)
      (`SceneComponent.K2_SetRelativeRotation` (`self.door2_Door2`) (`KismetMathLibrary.MakeRotator` 0.0 0.0 _returnvalue) false false))))

(fn `UserConstructionScript`)
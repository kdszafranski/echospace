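; BP_Chain is a level object that animates a continuously moving chain together with a linked cog.
; A timeline started on BeginPlay offsets the root vertically from its start position by MoveDelta and sets the referenced MyCog's pitch from the same curve value scaled by CogSpeed.
; When the timeline finishes, the root snaps back to its start position and playback restarts, creating an endless loop.
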(event `self.ReceiveBeginPlay`
  (bind (_startpos_x _startpos_y _startpos_z) (`KismetMathLibrary.BreakVector` (`self.StartPos`)))
  (bind _defaultsceneroot (`self.DefaultSceneRoot`))
  (bind _defaultsceneroot_2 (`/Game/Blueprints/LevelObjects/BP_Cog.DefaultSceneRoot` (`self.MyCog`)))
  (bind (_returnvalue_roll _returnvalue_pitch _returnvalue_yaw) (`KismetMathLibrary.BreakRotator` (`SceneComponent.K2_GetComponentRotation` _defaultsceneroot_2)))
  (set `self.StartPos` (`SceneComponent.K2_GetComponentLocation` _defaultsceneroot))
  (bind (_direction _dickchainy) (`Timeline|ChaineyChainChaaaaain` :!label _label)
    (:`Update`
      (`SceneComponent.K2_SetWorldLocation` _defaultsceneroot (`KismetMathLibrary.MakeVector` _startpos_x _startpos_y (+ _startpos_z (* _dickchainy (`self.MoveDelta`)))) true false)
      (`SceneComponent.K2_SetWorldRotation` _defaultsceneroot_2 (`KismetMathLibrary.MakeRotator` _returnvalue_roll (* (`self.CogSpeed`) _dickchainy) _returnvalue_yaw) false false))
    (:`Finished`
      (`SceneComponent.K2_SetWorldLocation` _defaultsceneroot (`self.StartPos`) false false)
      (goto _label :!via `PlayFromStart`))))

(fn `UserConstructionScript`)
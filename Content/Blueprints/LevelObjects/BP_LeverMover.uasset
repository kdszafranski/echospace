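; Lever level object that, when its action is performed, sends its stored location to the BP_MoverManager as the new move location.
; PerformAction triggers CallMover, which finds the manager by class lookup and passes it MyLocation.
; Activate switches the lever mesh's pitch between its two positions, briefly flashing a locked-slider material before changing to brushed nickel when activated.
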(event `Activate`
  (params (Activated :type Boolean))
  (bind _lever00_cube_001 (`self.lever00_Cube_001`))
  (if Activated
    (`SceneComponent.K2_SetRelativeRotation` _lever00_cube_001 (`KismetMathLibrary.MakeRotator` 0.0) false false)
    (`PrimitiveComponent.SetMaterial` _lever00_cube_001 0 "/Game/Materials00/MT_SliderLocked.MT_SliderLocked")
    (`KismetSystemLibrary.Delay` 0.2)
    (`PrimitiveComponent.SetMaterial` _lever00_cube_001 0 "/Game/StarterContent/Materials/M_Metal_Brushed_Nickel.M_Metal_Brushed_Nickel")
    (else
      (`SceneComponent.K2_SetRelativeRotation` _lever00_cube_001 (`KismetMathLibrary.MakeRotator` 0.0 90.0) false false))))

(event `/Game/Blueprints/BPI_Actions.PerformAction`
  ;[0 1 0.1856] TAKE ACTION
  (`self.CallMover`)
  (`KismetSystemLibrary.Delay` 0.6))

(event `CallMover`
  (bind _returnvalue (`GameplayStatics.GetActorOfClass` "/Game/Blueprints/LevelObjects/BP_MoverManager.BP_MoverManager_C"))
  (`/Game/Blueprints/LevelObjects/BP_MoverManager.SetMoveLocation` _returnvalue (`self.myLocation`)))

(fn `UserConstructionScript`)
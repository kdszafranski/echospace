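; BP_MoverManager is a level-object manager that slides a linked mover actor between two positions along the world Y axis and keeps two levers in sync with it.
; Tick eases the mover toward the current target Y with VInterpTo while leaving X and Z unchanged.
; SetMoveLocation with a non-negative index moves it and activates both levers, then returns both to the default state after a short delay.
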(event `self.ReceiveBeginPlay`
  (`self.SetMoveLocation` -1))

(event `self.ReceiveTick`
  (params (DeltaSeconds :type "Float (single-precision)"))
  (bind _currentlocation (`self.currentLocation`))
  (bind _defaultsceneroot (`/Game/Blueprints/LevelObjects/BP_Platform.DefaultSceneRoot` (`self.moverBP`)))
  (bind (_returnvalue_x _returnvalue_y _returnvalue_z) (`KismetMathLibrary.BreakVector` (`SceneComponent.K2_GetComponentLocation` _defaultsceneroot)))
  (if (> (`KismetMathLibrary.Abs` (- _returnvalue_y _currentlocation)) 0.1)
    (`SceneComponent.K2_SetWorldLocation` _defaultsceneroot (`KismetMathLibrary.VInterpTo` (`KismetMathLibrary.MakeVector` _returnvalue_x _returnvalue_y _returnvalue_z) (`KismetMathLibrary.MakeVector` _returnvalue_x _currentlocation _returnvalue_z) DeltaSeconds 3.0) false false)))

(event `SetMoveLocation`
  (params (LocationIndex :type Integer))
  (bind _lever0 (`self.Lever0`))
  (bind _lever1 (`self.Lever1`))
  (if (>= LocationIndex 0)
    (set `self.currentLocation` 1200.0)
    (`/Game/Blueprints/LevelObjects/BP_LeverMover.Activate` _lever0 true)
    (`/Game/Blueprints/LevelObjects/BP_LeverMover.Activate` _lever1 true)
    (`KismetSystemLibrary.Delay` 3.0)
    (`self.SetMoveLocation` -1)
    (else
      (set `self.currentLocation` 2900.0)
      (`/Game/Blueprints/LevelObjects/BP_LeverMover.Activate` _lever0 false)
      (`/Game/Blueprints/LevelObjects/BP_LeverMover.Activate` _lever1 false))))

(fn `UserConstructionScript`)
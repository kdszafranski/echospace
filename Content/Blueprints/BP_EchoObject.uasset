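; BP_EchoObject is a short-lived echo actor that ends itself on a fixed timer and leaves a BP_EchoEnd actor in its place.
; A few seconds after BeginPlay it calls EndInTwoSeconds, which plays the SNDEchoEnd sound.
; After a further short delay, that event spawns BP_EchoEnd at the root component's world location and destroys the actor.
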(event `self.ReceiveBeginPlay`
  (`KismetSystemLibrary.Delay` 3.0)
  (`self.EndInTwoSeconds`))

(event `EndInTwoSeconds`
  (`AudioComponent.Play` (`self.SND_EchoEnd`) 0.0)
  (`KismetSystemLibrary.Delay` 2.0)
  (`|SpawnActorFromClass` "/Game/Blueprints/FX/BP_EchoEnd.BP_EchoEnd_C" (`KismetMathLibrary.MakeTransform` (`SceneComponent.K2_GetComponentLocation` (`self.DefaultSceneRoot`))) "Undefined" "MultiplyWithRoot" null null)
  (`self.K2_DestroyActor`))

(fn `UserConstructionScript`)